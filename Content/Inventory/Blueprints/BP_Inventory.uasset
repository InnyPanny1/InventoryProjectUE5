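; BP_Inventory manages a slot-based item inventory with stacking and splitting, and creates the HUD that displays it.
; AddItem checks the weight limit, then looks for a partial stack or empty slot in the SItem array.
; MoveItem places or merges stacks, or opens a W_Split popup whose amount feeds SplitItem.
; Edits refresh the W_InventorySlot grid, and OpenInventory toggles visibility, cursor and input mode.
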(event Custom|InitializeInventory
  (bind _returnvalue (UserInterface|CreateWidget "/Game/Inventory/HUD/W_HUD.W_HUD_C"))
  (Variables|Default|SetHUD_Ref _returnvalue)
  (UserInterface|Viewport|AddtoViewport _returnvalue 0))

(event Custom|OpenInventory
  (bind _returnvalue (Game|GetPlayerController 0))
  (bind _returnvalue_2 (Game|GetPlayerController 0))
  (bind _hud_ref (Variables|Default|GetHUD_Ref))
  (bind _hud_ref_2 (Variables|Default|GetHUD_Ref))
  (if (Variables|Default|GetInventoryOpen?)
    (Variables|Default|SetInventoryOpen? false)
    (Variables|/Game/Inventory/HUD/W_HUD.W_HUD_C|SetInventoryVisibility _hud_ref_2 "Hidden")
    (Input|SetInputModeGameOnly _returnvalue)
    (Variables|/Script/Engine.PlayerController|SetbShowMouseCursor _returnvalue false)
    (else
      (Variables|Default|SetInventoryOpen? true)
      (Variables|/Game/Inventory/HUD/W_HUD.W_HUD_C|SetInventoryVisibility _hud_ref_2 "Visible")
      (Input|SetInputModeGameandUI _returnvalue_2 _hud_ref "DoNotLock" true)
      (Variables|/Script/Engine.PlayerController|SetbShowMouseCursor _returnvalue_2 true)
      (Class|Widget|SetUserFocus (Variables|/Game/Inventory/HUD/W_HUD.W_HUD_C|GetW_Inventory _hud_ref) _returnvalue_2))))

(event Custom|CallSplit
  (params (DragFrom :type Integer) (DragTo :type Integer) (Item :type S%20Item%20Structure))
  (bind _returnvalue (UserInterface|CreateWidget "/Game/Inventory/HUD/W_Split.W_Split_C"))
  (bind _output_get (Variables|Default|SetW_Split _returnvalue))
  (UserInterface|Viewport|AddtoViewport _output_get 0)
  (Default|SetInfo (Variables|Default|GetW_Split) Item)
  (EventDispatchers|BindEventtoCallSplit (Variables|Default|GetW_Split) (delegate Custom|SplitAmount)))

(event Custom|SplitAmount
  (params (AmountToSplit :type Integer))
  (CallFunction|SplitItem (stale Custom|CallSplit DragFrom) (stale Custom|CallSplit DragTo) AmountToSplit))

(event EventBeginPlay
  (CallFunction|InitializeInventory))

(event EventTick
  (params (DeltaSeconds :type Float%20%28single-precision%29)))

(fn AddItem
  (params (Item%20In :type S%20Item%20Structure))
  (bind (_id _itemname _itemcount _stackable_ _maxstack _weight) (Utilities|Struct|BreakS_Item Item%20In))
  (LocalVariables|SetItem%20L Item%20In)
  (LocalVariables|SetItem%20ID _id)
  (LocalVariables|SetItem%20Name _itemname)
  (LocalVariables|SetItem%20Count _itemcount)
  (LocalVariables|SetItem%20Stackable _stackable_)
  (LocalVariables|SetMax%20Stackable _maxstack)
  (LocalVariables|SetItem%20Weight _weight)
  (if (<= (+ (Variables|Default|GetCurrent%20Weight) (LocalVariables|GetItem%20Weight)) (Variables|Default|GetMax%20Weight))
    (bind (_array_element _array_index) (Utilities|Array|ForEachLoopwithBreak (Variables|Default|GetInventory) :!label _label)
      (:LoopBody
        (LocalVariables|SetArray%20%20Item _array_element)
        (LocalVariables|SetArray%20Item%20Index _array_index)
        (if (LocalVariables|GetItem%20Stackable)
          (bind _stack_index (Utilities|HasPartialStack (LocalVariables|GetItem%20L))
            (:True
              (LocalVariables|SetNew%20Item%20Index _stack_index)
              (LocalVariables|SetStack%20Remain (+ (.ItemCount (Utilities|Struct|BreakS_Item (Utilities|Array|Get(acopy) (Variables|Default|GetInventory) _stack_index))) (LocalVariables|GetItem%20Count)))
              (Development|PrintString (Utilities|String|ToString(Integer) (.ItemCount (Utilities|Struct|BreakS_Item (Utilities|Array|Get(acopy) (Variables|Default|GetInventory) _stack_index)))))
              (Utilities|FlowControl|Sequence
                (:then_0
                  (goto _label Break))
                (:then_1
                  (Utilities|Array|SetArrayElem (Variables|Default|GetInventory) (LocalVariables|GetNew%20Item%20Index) (LocalVariables|GetItem%20L) :!label _label_2)
                  (CallFunction|SetNewIndex (Utilities|Array|Get(acopy) (Variables|Default|GetInventory) (LocalVariables|GetNew%20Item%20Index)) (LocalVariables|GetNew%20Item%20Index))
                  (CallFunction|SetNewCount (Utilities|Array|Get(acopy) (Variables|Default|GetInventory) (LocalVariables|GetNew%20Item%20Index)) (LocalVariables|GetNew%20Item%20Index) (LocalVariables|GetStack%20Remain))
                  (CallFunction|RefreshInventorySlots))))
            (:False
              (if (Utilities|Enum|Equal(Enum) (.ID (Utilities|Struct|BreakS_Item (LocalVariables|GetArray%20%20Item))) (LocalVariables|GetItem%20ID))
                (if (<= (+ (.ItemCount (Utilities|Struct|BreakS_Item (LocalVariables|GetArray%20%20Item))) (LocalVariables|GetItem%20Count)) (LocalVariables|GetMax%20Stackable))
                  (LocalVariables|SetSpace%20Found true)
                  (LocalVariables|SetNew%20Item%20Index (LocalVariables|GetArray%20Item%20Index))
                  (LocalVariables|SetStack%20Remain (+ (.ItemCount (Utilities|Struct|BreakS_Item (LocalVariables|GetArray%20%20Item))) (LocalVariables|GetItem%20Count)))
                  (Development|PrintString "CAN STACK")
                  (goto _label Break)
                  (else
                    (Development|PrintString "NO MROE STACK POSSIBLME")))
                (elif (Utilities|Array|IsEmpty (.ItemName (Utilities|Struct|BreakS_Item (LocalVariables|GetArray%20%20Item))))
                  (Development|PrintString "ASSIGN TO NEW SLOT")
                  (LocalVariables|SetSpace%20Found true)
                  (LocalVariables|SetStack%20Remain (LocalVariables|GetItem%20Count))
                  (LocalVariables|SetNew%20Item%20Index (LocalVariables|GetArray%20Item%20Index))
                  (goto _label Break)
                  (else
                    (Development|PrintString "TOUTES LES SLOTS PRISES")
                    (LocalVariables|SetSpace%20Found false)
                    (LocalVariables|SetNew%20Item%20Index 0)
                    (LocalVariables|SetArray%20%20Item ""))))))))
      (:Completed
        (if (LocalVariables|GetSpace%20Found)
          (goto _label_2))))
    (else
      (return false ""))))

(fn RefreshInventorySlots
  (bind _hud_ref (Variables|Default|GetHUD_Ref))
  (bind _w_inventory (Variables|/Game/Inventory/HUD/W_HUD.W_HUD_C|GetW_Inventory _hud_ref))
  (bind _gridpanel_155 (Variables|/Game/Inventory/HUD/W_Inventory.W_Inventory_C|GetGridPanel_155 _w_inventory))
  (for _index (range 0 (Class|PanelWidget|GetChildrenCount _gridpanel_155))
    (bind _asw_inventory_slot (Utilities|Casting|CastToW_InventorySlot (Class|PanelWidget|GetChildat _gridpanel_155 _index)))
    (Default|RefreshSlot _asw_inventory_slot (Utilities|Array|Get(acopy) (Variables|Default|GetInventory) _index))))

(fn SetNewCount
  (params (Item%20Ref :type S%20Item%20Structure%20%28by%20ref%29) (Index :type Integer) (Item%20Count :type Integer))
  (bind _structout (Utilities|Struct|SetmembersinS_Item Item%20Ref Item%20Count))
  (Utilities|Array|SetArrayElem (Variables|Default|GetInventory) Index _structout))

(fn MoveItem
  (params (Index%20Drag%20Slot :type Integer) (Index%20Drop%20Slot :type Integer) (Split%20? :type Boolean))
  (bind _inventory (Variables|Default|GetInventory))
  (bind _inventory_2 (Variables|Default|GetInventory))
  (bind _inventory_3 (Variables|Default|GetInventory))
  (bind _output (Utilities|Array|Get(acopy) _inventory_3 Index%20Drop%20Slot))
  (bind _output_2 (Utilities|Array|Get(acopy) _inventory Index%20Drag%20Slot))
  (bind _output_3 (Utilities|Array|Get(acopy) _inventory_2 Index%20Drop%20Slot))
  (bind _itemcount (Utilities|Struct|BreakS_Item _output_2))
  (bind (_itemcount_2 _maxstack) (Utilities|Struct|BreakS_Item _output_3))
  (bind _returnvalue (+ _itemcount_2 _itemcount))
  (LocalVariables|SetItem%20In%20L (Utilities|Array|Get(acopy) (Variables|Default|GetInventory) Index%20Drag%20Slot))
  (LocalVariables|SetArray%20Item%20L (Utilities|Array|Get(acopy) (Variables|Default|GetInventory) Index%20Drop%20Slot))
  (LocalVariables|SetSlot%20Index%20L Index%20Drop%20Slot)
  (if Split%20?
    (if (Utilities|Array|IsEmpty (Utilities|Struct|BreakS_Item (LocalVariables|GetArray%20Item%20L)))
      (CallFunction|CallSplit Index%20Drag%20Slot Index%20Drop%20Slot (Utilities|Array|Get(acopy) (Variables|Default|GetInventory) Index%20Drag%20Slot)))
    (else
      ;[0 0.9297 1] Check slot empty
      (if (Utilities|Array|IsEmpty (Utilities|Struct|BreakS_Item (LocalVariables|GetArray%20Item%20L)))
        (Utilities|Array|SetArrayElem (Variables|Default|GetInventory) (LocalVariables|GetSlot%20Index%20L) (LocalVariables|GetItem%20In%20L))
        (CallFunction|SetNewIndex (LocalVariables|GetItem%20In%20L) (LocalVariables|GetSlot%20Index%20L))
        (CallFunction|RefreshInventorySlots)
        (return true)
        (elif (Utilities|Enum|Equal(Enum) (.ID (Utilities|Struct|BreakS_Item (LocalVariables|GetItem%20In%20L))) (.ID (Utilities|Struct|BreakS_Item (LocalVariables|GetArray%20Item%20L))))
          ;[0.9219 1 0] Check for stack
          (if (Utilities|Struct|BreakS_Item (Utilities|Array|Get(acopy) (Variables|Default|GetInventory) Index%20Drag%20Slot))
            (if (> _returnvalue _maxstack)
              (return false)
              (else
                (Utilities|Array|SetArrayElem (Variables|Default|GetInventory) (LocalVariables|GetSlot%20Index%20L) _output)
                (CallFunction|SetNewIndex _output (LocalVariables|GetSlot%20Index%20L))
                (CallFunction|SetNewCount _output (LocalVariables|GetSlot%20Index%20L) _returnvalue)
                (CallFunction|RefreshInventorySlots)
                (return true)))
            (else
              (return false)))
          (else
            (return false)))))))

(fn RemoveItem
  (params (Index :type Integer))
  (Utilities|Array|SetArrayElem (Variables|Default|GetInventory) Index (Utilities|Struct|MakeS_Item "" "" 1 false 0 0 0.0 false 0 Index))
  (CallFunction|RefreshInventorySlots))

(fn SetNewIndex
  (params (Item%20Ref :type S%20Item%20Structure%20%28by%20ref%29) (Index :type Integer))
  (bind _structout (Utilities|Struct|SetmembersinS_Item Item%20Ref Index))
  (Utilities|Array|SetArrayElem (Variables|Default|GetInventory) Index _structout))

(fn FindFreeSlot)

(fn SplitItem
  (params (Index%20Drag%20Slot :type Integer) (Index%20Drop%20Slot :type Integer) (New%20Count :type Integer))
  (bind _inventory (Variables|Default|GetInventory))
  (bind _inventory_2 (Variables|Default|GetInventory))
  (bind _output (Utilities|Array|Get(acopy) _inventory_2 Index%20Drop%20Slot))
  (bind _output_2 (Utilities|Array|Get(acopy) _inventory Index%20Drop%20Slot))
  (bind (_itemcount _maxstack) (Utilities|Struct|BreakS_Item _output_2))
  (bind _structout (Utilities|Struct|SetmembersinS_Item (Utilities|Array|Get(acopy) (Variables|Default|GetInventory) Index%20Drag%20Slot) New%20Count))
  (LocalVariables|SetItem%20In%20L _structout)
  (LocalVariables|SetArray%20Item%20L (Utilities|Array|Get(acopy) (Variables|Default|GetInventory) Index%20Drop%20Slot))
  (LocalVariables|SetSlot%20Index%20L Index%20Drop%20Slot)
  ;[0 0.9297 1] Check slot empty
  (if (Utilities|Array|IsEmpty (Utilities|Struct|BreakS_Item (LocalVariables|GetArray%20Item%20L)))
    (Utilities|Array|SetArrayElem (Variables|Default|GetInventory) (LocalVariables|GetSlot%20Index%20L) (LocalVariables|GetItem%20In%20L))
    (CallFunction|SetNewIndex (LocalVariables|GetItem%20In%20L) (LocalVariables|GetSlot%20Index%20L))
    (CallFunction|SetNewCount (LocalVariables|GetItem%20In%20L) Index%20Drag%20Slot (- (Utilities|Struct|BreakS_Item (LocalVariables|GetItem%20In%20L)) New%20Count))
    (CallFunction|RefreshInventorySlots)
    (return true)
    (else
      ;[0.4297 0 1] Check if slot hit is the same ID
      (if (Utilities|Enum|Equal(Enum) (.ID (Utilities|Struct|BreakS_Item (LocalVariables|GetItem%20In%20L))) (.ID (Utilities|Struct|BreakS_Item (LocalVariables|GetArray%20Item%20L))))
        ;[0.9219 1 0] Check for stack
        (if (Utilities|Struct|BreakS_Item (LocalVariables|GetItem%20In%20L))
          (if (> (+ _itemcount (Utilities|Struct|BreakS_Item (LocalVariables|GetItem%20In%20L))) _maxstack)
            (return false)
            (else
              (Utilities|Array|SetArrayElem (Variables|Default|GetInventory) (LocalVariables|GetSlot%20Index%20L) _output)
              (CallFunction|SetNewIndex _output (LocalVariables|GetSlot%20Index%20L))
              (CallFunction|SetNewCount _output (LocalVariables|GetSlot%20Index%20L) (+ _itemcount (Utilities|Struct|BreakS_Item (LocalVariables|GetItem%20In%20L))))
              (CallFunction|RefreshInventorySlots)
              (return true)))
          (else
            (return false)))
        (else
          (return false))))))