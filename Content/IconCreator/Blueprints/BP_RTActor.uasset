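; Icon-creator stage actor that frames a mesh and saves scene captures as static textures.
; Mouse input rotates, pans, zooms and resets the X/Y pivot components, with the background plane following zoom.
; BeginPlay creates dynamic background and outline materials, feeding the outline and unit-background ones into post-process.
; CaptureTexture renders to a temporary sized target with FOV correction for vertical images, saves it editor-only, then restores RT_Image and FOV.
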(event Custom|CaptureTexture
  (params (Width :type Integer) (Height :type Integer) (Name :type String) (Vertical? :type Boolean))
  (bind _returnvalue (Rendering|CreateRenderTarget2D Width Height "RTF_RGBA8"))
  (Variables|Default|SetOriginal%20Fov (Variables|/Script/Engine.SceneCaptureComponent2D|GetFOVAngle (Variables|Default|GetSceneCaptureComponent2D)))
  (if Vertical?
    (Variables|/Script/Engine.SceneCaptureComponent2D|SetFOVAngle (Variables|Default|GetSceneCaptureComponent2D) (+ (* (Variables|/Script/Engine.SceneCaptureComponent2D|GetFOVAngle (Variables|Default|GetSceneCaptureComponent2D)) (/ (Math|Conversions|ToFloat(Integer) Width) (Math|Conversions|ToFloat(Integer) Height))) 0.85)))
  (bind _output_get (Variables|/Script/Engine.SceneCaptureComponent2D|SetTextureTarget (Variables|Default|GetSceneCaptureComponent2D) _returnvalue))
  (Variables|/Script/Engine.SceneCaptureComponent|SetbCaptureEveryFrame (Variables|Default|GetSceneCaptureComponent2D) true)
  (Rendering|SceneCapture|CaptureScene (Variables|Default|GetSceneCaptureComponent2D) :!class /Script/Engine.SceneCaptureComponent2D)
  (Class|KismetRenderingLibrary|RenderTargetCreateStaticTexture2DEditorOnly _output_get Name "TC_Default" "TMGS_FromTextureGroup")
  (Variables|/Script/Engine.SceneCaptureComponent|SetbCaptureEveryFrame (Variables|Default|GetSceneCaptureComponent2D) false)
  (Variables|/Script/Engine.SceneCaptureComponent2D|SetTextureTarget (Variables|Default|GetSceneCaptureComponent2D) "/Game/IconCreator/Textures/RT_Image.RT_Image")
  (Variables|/Script/Engine.SceneCaptureComponent|SetbCaptureEveryFrame (Variables|Default|GetSceneCaptureComponent2D) true)
  (Variables|/Script/Engine.SceneCaptureComponent2D|SetFOVAngle (Variables|Default|GetSceneCaptureComponent2D) (Variables|Default|GetOriginal%20Fov)))

(event Custom|ResetTransform
  (Transformation|SetRelativeRotation (Variables|Default|GetX) "0,90.000000, 0" false false)
  (Transformation|SetRelativeRotation (Variables|Default|GetY) "0, 0, 0" false false)
  (Transformation|SetRelativeLocation (Variables|Default|GetX) "0, 0, 0" false false))

(event EventBeginPlay
  (bind _returnvalue (Rendering|Material|CreateDynamicMaterialInstance "/Game/IconCreator/Materials/M_BackgroundPlane.M_BackgroundPlane" "None" "None" :!class /Script/Engine.KismetMaterialLibrary))
  (bind _output_get (Variables|Default|SetPlanDM _returnvalue))
  (Rendering|Material|SetMaterial (Variables|Default|GetSM_BackgroundPlane) 0 _output_get)
  (Input|EnableInput (Game|GetPlayerController 0))
  (bind _returnvalue_2 (Rendering|Material|CreateDynamicMaterialInstance "/Game/IconCreator/Materials/PP_Outliner_M.PP_Outliner_M" "None" "None" :!class /Script/Engine.KismetMaterialLibrary))
  (bind _output_get_2 (Variables|Default|SetDM _returnvalue_2))
  (Rendering|Material|SetScalarParameterValue (Variables|Default|GetDM) "OutLineThickness" 1.0 :!class /Script/Engine.MaterialInstanceDynamic)
  (Rendering|Material|SetVectorParameterValue (Variables|Default|GetDM) "OutlineColor" "(R=1.000000,G=1.000000,B=1.000000,A=1.000000)" :!class /Script/Engine.MaterialInstanceDynamic)
  (bind _returnvalue_3 (Rendering|Material|CreateDynamicMaterialInstance "/Game/IconCreator/Materials/M_BackgroundPlane_Unit.M_BackgroundPlane_Unit" "None" "None" :!class /Script/Engine.KismetMaterialLibrary))
  (bind _output_get_3 (Variables|Default|SetPlan_DM_Unit _returnvalue_3))
  (Utilities|Array|AppendArray (Variables|Default|GetPostProcess%20Materials) (Utilities|Array|MakeArray (Utilities|Struct|MakeWeightedBlendable 1.0 _output_get_2) (Utilities|Struct|MakeWeightedBlendable 1.0 _output_get_3)))
  (bind _structout (Utilities|Struct|SetmembersinPostProcessSettings (Variables|/Script/Engine.PostProcessComponent|GetSettings (Variables|Default|GetPostProcess)) "Lumen" "Lumen" (Utilities|Struct|MakeWeightedBlendables (Variables|Default|GetPostProcess%20Materials))))
  (Variables|/Script/Engine.PostProcessComponent|SetSettings (Variables|Default|GetPostProcess) _structout))

(event EventTick
  (params (DeltaSeconds :type Float%20%28single-precision%29))
  (bind _movespeed (Variables|Default|GetMoveSpeed))
  (if (Variables|Default|GetMove?)
    (Transformation|AddRelativeLocation (Variables|Default|GetX) (Math|Vector|MakeVector 0.0 (* (Class|Actor|GetInputAxisKeyValue) _movespeed) (* (Class|Actor|GetInputAxisKeyValue) _movespeed)) false false)))

(event Input|MouseEvents|MouseX
  (params (AxisValue :type Float%20%28single-precision%29))
  ;[1 1 1] When mouse move with click, rotate weapon mesh
  (if (Variables|Default|GetStartRotation)
    (Transformation|AddLocalRotation (Variables|Default|GetX) (Math|Rotator|MakeRotator 0.0 0.0 (* AxisValue -0.5)) false false)))

(event Input|MouseEvents|MouseY
  (params (AxisValue :type Float%20%28single-precision%29))
  ;[1 1 1] When mouse move with click, rotate weapon mesh
  (if (Variables|Default|GetStartRotation)
    (Transformation|AddWorldRotation (Variables|Default|GetY) (Math|Rotator|MakeRotator 0.0 (* AxisValue -0.5) 0.0) false false)))

(event Input|MouseEvents|MouseWheelDown
  (params (Key :type Key%20Structure :default "None"))
  (bind _x (Variables|Default|GetX))
  (bind _relativelocation (Variables|/Script/Engine.SceneComponent|GetRelativeLocation _x))
  (:Pressed
    (bind _output_get (Variables|Default|SetActorScale (Math|Vector|MakeVector (- (.x _relativelocation) (Variables|Default|GetZoomSpeed)) (.y _relativelocation) (.z _relativelocation))))
    (Transformation|SetRelativeLocation (Variables|Default|GetX) _output_get false false)
    (Transformation|SetRelativeLocation (Variables|Default|GetSM_BackgroundPlane) (+ _output_get (Variables|Default|GetBackPlanDistance)) false false)))

(event Input|MouseEvents|MouseWheelUp
  (params (Key :type Key%20Structure :default "None"))
  (bind _x (Variables|Default|GetX))
  (bind _relativelocation (Variables|/Script/Engine.SceneComponent|GetRelativeLocation _x))
  (:Pressed
    (bind _output_get (Variables|Default|SetActorScale (Math|Vector|MakeVector (+ (.x _relativelocation) (Variables|Default|GetZoomSpeed)) (.y _relativelocation) (.z _relativelocation))))
    (Transformation|SetRelativeLocation (Variables|Default|GetX) _output_get false false)
    (Transformation|SetRelativeLocation (Variables|Default|GetSM_BackgroundPlane) (+ _output_get (Variables|Default|GetBackPlanDistance)) false false)))

(event Input|MouseEvents|MiddleMouseButton
  (params (Key :type Key%20Structure :default "None"))
  (:Pressed
    (Variables|Default|SetStartRotation false)
    (Variables|Default|SetMove? true))
  (:Released
    (Variables|Default|SetMove? false)))

(event Input|MouseEvents|RightMouseButton
  (params (Key :type Key%20Structure :default "None"))
  (:Pressed
    (Transformation|SetRelativeRotation (Variables|Default|GetX) "0,90.000000, 0" false false)
    (Transformation|SetRelativeRotation (Variables|Default|GetY) "0, 0, 0" false false)
    (Transformation|SetRelativeLocation (Variables|Default|GetX) "0, 0, 0" false false)))

(fn ConstructionScript
  (bind _structout (Utilities|Struct|SetmembersinPostProcessSettings (Variables|/Script/Engine.PostProcessComponent|GetSettings (Variables|Default|GetPostProcess)) (Utilities|Struct|MakeWeightedBlendables (Variables|Default|GetPostProcess%20Materials))))
  (Variables|/Script/Engine.PostProcessComponent|SetSettings (Variables|Default|GetPostProcess) _structout))